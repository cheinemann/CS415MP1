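; Projectile actor that flies down the tunnel and scores points for the player when it hits a sphere enemy.
; Tick sweeps it along world X at twice the BPPlayer forward speed.
; On overlap it identifies the BP_Tunnel component hit, passing through the trigger zone and destroying itself on anything else, with debug prints.
; Only SphereEnemy hits increase the score, and overlaps with non-tunnel actors are ignored.
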(event OnComponentBeginOverlap(Projectile)
  (params (OverlappedComponent :type Primitive%20Component%20Object%20Reference) (OtherActor :type Actor%20Object%20Reference) (OtherComp :type Primitive%20Component%20Object%20Reference) (OtherBodyIndex :type Integer) (bFromSweep :type Boolean) (SweepResult :type Hit%20Result%20Structure%20%28by%20ref%29))
  ;[1 1 1] All different conditions for if projectile hits something
  (Development|PrintString "Collision")
  (bind _asbp_tunnel (Utilities|Casting|CastToBP_Tunnel OtherActor))
  (if (== OtherComp (Variables|/Game/InfiniteMatrix/Blueprints/BP_Tunnel.BP_Tunnel_C|GetWallMesh _asbp_tunnel))
    (Development|PrintString "Hit wall")
    (Actor|DestroyActor)
    (else
      (Development|PrintString "Didn't hit wall")
      (if (not (== (Variables|/Game/InfiniteMatrix/Blueprints/BP_Tunnel.BP_Tunnel_C|GetTriggerZone _asbp_tunnel) OtherComp))
        (if (== (Variables|/Game/InfiniteMatrix/Blueprints/BP_Tunnel.BP_Tunnel_C|GetCube_health _asbp_tunnel) OtherComp)
          (Actor|DestroyActor)
          (elif (== (Variables|/Game/InfiniteMatrix/Blueprints/BP_Tunnel.BP_Tunnel_C|GetSphere_enemy _asbp_tunnel) OtherComp)
            (Default|IncreaseScore (Variables|Default|GetBP_Player))
            (Actor|DestroyActor)
            (else
              (Actor|DestroyActor))))))))

(event EventBeginPlay)

(event Collision|EventActorBeginOverlap
  (params (OtherActor :type Actor%20Object%20Reference)))

(event EventTick
  (params (DeltaSeconds :type Float%20%28single-precision%29))
  ;[1 1 1] Move projectile forward
  (Transformation|AddActorWorldOffset (Math|Vector|MakeVector (* DeltaSeconds (* 2.0 (Variables|/Game/InfiniteMatrix/Blueprints/BP_Player.BP_Player_C|GetForwardSpeed (Variables|Default|GetBP_Player)))) 0.0 0.0) true))

(fn ConstructionScript)