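; Tunnel segment for an endless runner: passing its trigger spawns the next segment via TunnelSpawner, destroys this one and raises player score.
; Tick spins the holed wall; hitting it deals damage, plays a sound and lowers score.
; A health cube heals the player, while an enemy sphere damages whatever overlaps it.
; Helper functions randomize wall mesh, rotation and pickup placement, but none are called within this Blueprint.
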(event OnComponentBeginOverlap(TriggerZone)
  (params (OverlappedComponent :type Primitive%20Component%20Object%20Reference) (OtherActor :type Actor%20Object%20Reference) (OtherComp :type Primitive%20Component%20Object%20Reference) (OtherBodyIndex :type Integer) (bFromSweep :type Boolean) (SweepResult :type Hit%20Result%20Structure%20%28by%20ref%29))
  ;[1 1 1] If pass through wall, increase score and destroy tunnel that was passed through
  (bind _asbp_player (Utilities|Casting|CastToBP_Player OtherActor))
  (Utilities|FlowControl|Sequence
    (:then_0
      (Default|SpawnTunnelatSpawnPoint (Variables|Default|GetTunnelSpawner))
      (Actor|DestroyActor))
    (:then_1
      (if (Variables|Default|GetPassThroughTriggerZone)
        (bind _asbp_player_2 (Utilities|Casting|CastToBP_Player (Game|Player|GetPlayerPawn 0)))
        (Variables|/Game/InfiniteMatrix/Blueprints/BP_Player.BP_Player_C|SetScore _asbp_player_2 (+ (Variables|/Game/InfiniteMatrix/Blueprints/BP_Player.BP_Player_C|GetScore _asbp_player_2) 1))))
    (:then_2
      (Default|IncreaseScore _asbp_player))))

(event OnComponentBeginOverlap(Cube_health)
  (params (OverlappedComponent :type Primitive%20Component%20Object%20Reference) (OtherActor :type Actor%20Object%20Reference) (OtherComp :type Primitive%20Component%20Object%20Reference) (OtherBodyIndex :type Integer) (bFromSweep :type Boolean) (SweepResult :type Hit%20Result%20Structure%20%28by%20ref%29))
  ;[1 1 1] If hit cube, increment health
  (bind _asbp_player (Utilities|Casting|CastToBP_Player (Game|Player|GetPlayerPawn 0)))
  (Default|HealPlayer _asbp_player))

(event OnComponentBeginOverlap(WallMesh)
  (params (OverlappedComponent :type Primitive%20Component%20Object%20Reference) (OtherActor :type Actor%20Object%20Reference) (OtherComp :type Primitive%20Component%20Object%20Reference) (OtherBodyIndex :type Integer) (bFromSweep :type Boolean) (SweepResult :type Hit%20Result%20Structure%20%28by%20ref%29))
  ;[1 1 1] If hit wall, decrease score
  (bind _asbp_player (Utilities|Casting|CastToBP_Player OtherActor))
  (Game|Damage|ApplyDamage _asbp_player 2e+01 0 0)
  (Audio|PlaySound2D "/Engine/EditorSounds/GamePreview/EjectFromPlayer_Cue.EjectFromPlayer_Cue" 1.0 1.0 0.0 0 0)
  (Default|DecreaseScore _asbp_player))

(event OnComponentBeginOverlap(Sphere_enemy)
  (params (OverlappedComponent :type Primitive%20Component%20Object%20Reference) (OtherActor :type Actor%20Object%20Reference) (OtherComp :type Primitive%20Component%20Object%20Reference) (OtherBodyIndex :type Integer) (bFromSweep :type Boolean) (SweepResult :type Hit%20Result%20Structure%20%28by%20ref%29))
  ;[1 1 1] If hit sphere, which is enemy, decrement health
  (Game|Damage|ApplyDamage OtherActor 2e+01 0 0)
  (Components|DestroyComponent (Variables|Default|GetSphere_enemy)))

(event EventBeginPlay
  (Transformation|AddLocalOffset (Variables|Default|GetCube_health) (Math|Vector|MakeVector (Math|Random|RandomFloatinRange 0.0 5e+02) 0.0 0.0) false false))

(event EventTick
  (params (DeltaSeconds :type Float%20%28single-precision%29))
  ;[1 1 1] Rotate walls
  (Transformation|AddLocalRotation (Variables|Default|GetWallMesh) (Math|Rotator|MakeRotator (* DeltaSeconds (Variables|Default|GetRotateSpeed)) 0.0 0.0) false false))

(fn ConstructionScript)

(fn RandomizeWall
  (Components|StaticMesh|SetStaticMesh (Variables|Default|GetWallMesh) (Utilities|Select :Index (Math|Random|RandomIntegerinRange 0 3) :Option%200 "/Game/InfiniteMatrix/Meshes/SM_Hole_01.SM_Hole_01" :Option%201 "/Game/InfiniteMatrix/Meshes/SM_Hole_02.SM_Hole_02" :Option%202 "/Game/InfiniteMatrix/Meshes/SM_Hole_03.SM_Hole_03" :Option%203 "/Game/InfiniteMatrix/Meshes/SM_Hole_04.SM_Hole_04"))
  (Transformation|AddLocalRotation (Variables|Default|GetWallMesh) (Math|Rotator|MakeRotator (Math|Random|RandomFloatinRange 0.0 3.6e+02) 0.0 0.0) false false))

(fn RandomizeHealthLocationOld
  (Components|StaticMesh|SetStaticMesh (Variables|Default|GetCube_health) 0)
  (Transformation|AddLocalOffset (Variables|Default|GetCube_health) (Math|Vector|MakeVector (Math|Random|RandomFloatinRange 1e+03 2.3e+03) 0.0 0.0) false false))

(fn RandomizeHealthLocation
  (if (== (Math|Random|RandomInteger 0) 0)
    (Class|SceneComponent|AddWorldTransform (Variables|Default|GetCube_health) (Math|Transform|MakeTransform (Math|Vector|MakeVector (Math|Random|RandomFloatinRange 1e+03 1.5e+03) (Math|Random|RandomFloatinRange -2.5e+02 3e+02) (Math|Random|RandomFloatinRange -2.5e+02 3e+02)) "0, 0, 0" "1.000000,1.000000,1.000000") false false)
    (else
      (Class|SceneComponent|AddWorldTransform (Variables|Default|GetCube_health) (Math|Transform|MakeTransform "0.000000,10000.000000,10000.000000" "0, 0, 0" "1.000000,1.000000,1.000000") false false))))

(fn RandomizeEnemyLocation
  (if (== (Math|Random|RandomInteger 0) 0)
    (Class|SceneComponent|AddWorldTransform (Variables|Default|GetSphere_enemy) (Math|Transform|MakeTransform (Math|Vector|MakeVector (Math|Random|RandomFloatinRange 1e+03 1.5e+03) (Math|Random|RandomFloatinRange -2.5e+02 3e+02) (Math|Random|RandomFloatinRange -2.5e+02 3e+02)) "0, 0, 0" "1.000000,1.000000,1.000000") false false)
    (else
      (Components|DestroyComponent (Variables|Default|GetSphere_enemy)))))